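; BP_Table is a table Blueprint that detects whether a BP_Chair is in place at it.
; Its TableCollision begin and end overlap events filter for BP_Chair, then set or clear the ChairInPlace flag on player 0's BP_GameCharacter.
; Both events print debug messages showing the change and the resulting flag value.
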(event `self.Table Collision.OnComponentBeginOverlap`
  (params (OverlappedComponent :type "PrimitiveComponent Object Reference") (OtherActor :type "Actor Object Reference") (OtherComp :type "PrimitiveComponent Object Reference") (OtherBodyIndex :type Integer) (bFromSweep :type Boolean) (SweepResult :type "HitResult Structure (by ref)"))
  (cast `/Game/Blueprints/BP_Chair` OtherActor)
  (`KismetSystemLibrary.PrintString` "Chair in place")
  (bind _asbp_game_character (cast `/Game/Blueprints/CharacterBlueprints/BP_GameCharacter` (`GameplayStatics.GetPlayerCharacter` 0)))
  (bind _output_get (set `/Game/Blueprints/CharacterBlueprints/BP_GameCharacter.ChairInPlace` true _asbp_game_character))
  (`KismetSystemLibrary.PrintString` (`KismetStringLibrary.Conv_BoolToString` _output_get)))

(event `self.Table Collision.OnComponentEndOverlap`
  (params (OverlappedComponent :type "PrimitiveComponent Object Reference") (OtherActor :type "Actor Object Reference") (OtherComp :type "PrimitiveComponent Object Reference") (OtherBodyIndex :type Integer))
  (cast `/Game/Blueprints/BP_Chair` OtherActor)
  (`KismetSystemLibrary.PrintString` "Chair Removed from Place")
  (bind _asbp_game_character (cast `/Game/Blueprints/CharacterBlueprints/BP_GameCharacter` (`GameplayStatics.GetPlayerCharacter` 0)))
  (bind _output_get (set `/Game/Blueprints/CharacterBlueprints/BP_GameCharacter.ChairInPlace` false _asbp_game_character))
  (`KismetSystemLibrary.PrintString` (`KismetStringLibrary.Conv_BoolToString` _output_get)))

(fn `UserConstructionScript`)