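; BP_FireBall is a moving fireball obstacle that travels either horizontally or vertically, chosen by MoveHorizontal.
; Horizontal fireballs move along world X in Tick, reversing Speed at plus or minus MaxX around the world origin.
; Vertical fireballs play a timeline from BeginPlay that offsets the initial location, with VerticalPositive selecting the positive or negative movement track.
; The graphs contain only movement, with no collision or damage logic.
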(event `self.ReceiveBeginPlay`
  (if (not (`self.Move Horizontal`))
    (set `self.Initial Location` (`self.K2_GetActorLocation`))
    (bind (_direction _y_movement_positive _y_movement_negative) (`Timeline|Fireball Vertical Movement`)
      (:`Update`
        (if (`self.Vertical Positive`)
          (`self.K2_SetActorLocation` (+ (`self.Initial Location`) _y_movement_positive))
          (else
            (`self.K2_SetActorLocation` (+ (`self.Initial Location`) _y_movement_negative))))))))

(event `self.ReceiveTick`
  (params (DeltaSeconds :type "Float (single-precision)"))
  (bind _returnvalue_x (`KismetMathLibrary.BreakVector` (`self.K2_GetActorLocation`)))
  (bind _returnvalue_x_2 (`KismetMathLibrary.BreakVector` (`self.K2_GetActorLocation`)))
  (bind (_returnvalue_x_3 _returnvalue_y _returnvalue_z) (`KismetMathLibrary.BreakVector` (`self.K2_GetActorLocation`)))
  (if (`self.Move Horizontal`)
    (`self.K2_SetActorLocation` (`KismetMathLibrary.MakeVector` (+ (* DeltaSeconds (`self.Speed`)) _returnvalue_x_3) _returnvalue_y _returnvalue_z))
    (if (>= _returnvalue_x_2 (`self.Max X`))
      (set `self.Speed` (* (`self.Speed`) -1.0))
      (elif (<= _returnvalue_x (* (`self.Max X`) -1.0))
        (set `self.Speed` (`KismetMathLibrary.Abs` (`self.Speed`)))))))

(fn `UserConstructionScript`)